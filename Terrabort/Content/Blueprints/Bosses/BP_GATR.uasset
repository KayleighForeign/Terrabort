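; GATR boss Blueprint that plays its wake-up and attack montages and fires callbacks when they end.
; Attack passes through HandleCooldown, which compares game time to the attack's last activation and writes the new timestamp back into the Attacks map by name.
; Completed and interrupted montages both signal the end, while a missing attack montage or active cooldown signals it after a short delay.
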(event Custom|Attack
  (params (Attack :type Struct%20GATR%20Attack%20Structure) (AttackName :type Name))
  (bind _animationmontage (Utilities|Struct|BreakStruct_GATR_Attack Attack))
  ;[1 1 1] Attack
  (Utilities|IsValid _animationmontage
    (:Is%20Valid
      ;[1 1 1] This one may not be needed at all... just in case I leave it here for a while just to be sure.
      (|HandleCooldown Attack AttackName
        (:Success
          (Animation|Montage|PlayMontage (Variables|Character|GetMesh) _animationmontage
            (:OnCompleted
              _)
            (:OnInterrupted
              _)))
        (:Fail
          (Utilities|FlowControl|Delay 0.1 :!label _label))))
    (:Is%20Not%20Valid
      (goto _label)))
  (Default|CallOnAttackEnd))

(event Custom|WakeUp
  (bind _wake_up_animation (Variables|Animations|GetWake%20up%20animation))
  ;[1 1 1] Wake up
  (Utilities|IsValid _wake_up_animation
    (:Is%20Valid
      (Animation|Montage|PlayMontage (Variables|Character|GetMesh) _wake_up_animation
        (:OnCompleted
          _)
        (:OnInterrupted
          _)))
    (:Is%20Not%20Valid
      _))
  (Default|CallOnWakeUpFinished))

(fn ConstructionScript)