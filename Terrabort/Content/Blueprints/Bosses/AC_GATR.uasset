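; AI controller for the GATR boss, handling perception and blackboard state changes.
; Perception updates run CanSenseActor on each updated actor and store the result in SensesActor, using only the first last-sensed stimulus.
; SetStatePassive and SetStateAttack write the AI state enum to the Blackboard, with attack also setting the target object.
; The perception event does not call either state setter itself.
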(event OnPerceptionUpdated(AIPerception)
  (params (UpdatedActors :type Array%20of%20Actor%20Object%20References))
  ;[1 1 1] Sensing
  (for _array_element UpdatedActors
    (bind _sense (CallFunction|CanSenseActor _array_element))
    (Variables|Default|SetSensesActor _sense)))

(fn ConstructionScript)

(fn SetStatePassive
  (AI|Components|Blackboard|SetValueasEnum (Variables|Default|GetBlackboard) (Variables|Default|GetState%20key%20name) (Utilities|Enum|LiteralenumEnum_AI_States "NewEnumerator0")))

(fn SetStateAttack
  (params (Attack%20Target :type Actor%20Object%20Reference))
  (AI|Components|Blackboard|SetValueasObject (Variables|Default|GetBlackboard) (Variables|Default|GetAttack%20target%20key%20name) Attack%20Target)
  (AI|Components|Blackboard|SetValueasEnum (Variables|Default|GetBlackboard) (Variables|Default|GetState%20key%20name) (Utilities|Enum|LiteralenumEnum_AI_States "NewEnumerator1")))

(fn CanSenseActor
  (params (Actor :type Actor%20Object%20Reference))
  (bind _info (Class|AIPerceptionComponent|GetActorsPerception (Variables|Default|GetAIPerception) Actor))
  (for _array_element (.LastSensedStimuli (Utilities|Struct|BreakActorPerceptionBlueprintInfo _info))
    (return (.bSuccessfullySensed (Utilities|Struct|BreakAIStimulus _array_element)))))